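; BP_Alien is an enemy character that chases and melee-attacks the player marine.
; An AIMoveTo loop repeatedly pursues the player, while Tick checks range and state, halting movement during the attack montage.
; DamagePlayer applies the hit but is not called within this Blueprint.
; Incoming damage reduces health; death credits the marine's kill, notifies BP_MarineGameMode, removes the capsule, and destroys the actor after a delay.
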(event EventBeginPlay
  (if (not (and (CallFunction|IsPlayerDead?) (Variables|Default|GetIs%20Alien%20Dead))) :!label _label
    (AI|AIMoveTo self "0, 0, 0" (Game|GetPlayerCharacter 0) 5.0 false
      (:OnSuccess
        _)
      (:OnFail
        _))
    (Utilities|FlowControl|Delay 0.2)
    (goto _label)))

(event EventTick
  (params (DeltaSeconds :type Float%20%28single-precision%29))
  (if (CallFunction|IsAbletoAttackPlayer?)
    (Components|Activation|Deactivate (Variables|Character|GetCharacterMovement))
    (Animation|Montage|PlayMontage (Variables|Character|GetMesh) "/Game/Characters/Enemy_Great_Spider/Animations/AnimM_AlienAttack.AnimM_AlienAttack"
      (:OnCompleted
        (Components|Activation|Activate (Variables|Character|GetCharacterMovement) false)))))

(event Game|Damage|EventAnyDamage
  (params (Damage :type Float%20%28single-precision%29) (DamageType :type Damage%20Type%20Object%20Reference) (InstigatedBy :type Controller%20Object%20Reference) (DamageCauser :type Actor%20Object%20Reference))
  (Utilities|DamageAlien Damage
    (:Alien%20Is%20Dead
      (Variables|Default|SetIs%20Alien%20Dead true)
      (CallFunction|KillAI)
      (Utilities|FlowControl|Delay 3.0)
      (Actor|DestroyActor))))

(fn ConstructionScript)

(fn IsWithinAttackRange?
  (return (<= (Transformation|GetDistanceTo (Game|GetPlayerCharacter 0)) (Variables|Default|GetAttack%20Range))))

(fn IsAttacking?
  (return (Animation|Montage|MontageIsPlaying (Components|SkeletalMesh|GetAnimInstance (Variables|Character|GetMesh)) "/Game/Characters/Enemy_Great_Spider/Animations/AnimM_AlienAttack.AnimM_AlienAttack")))

(fn DamagePlayer
  (Game|Damage|ApplyDamage (Game|GetPlayerCharacter 0) (Variables|Default|GetDamage) 0 0))

(fn IsPlayerDead?
  (bind _asbp_marine (Utilities|Casting|CastToBP_Marine (Game|GetPlayerCharacter 0)))
  (return (Variables|/Game/Blueprints/Pawns/Marine/BP_Marine.BP_Marine_C|GetIs%20Dead _asbp_marine)))

(fn IsAbletoAttackPlayer?
  (return (Math|Boolean|ANDBoolean (CallFunction|IsWithinAttackRange?) (not (CallFunction|IsAttacking?)) (not (CallFunction|IsPlayerDead?)) (not (Variables|Default|GetIs%20Alien%20Dead)))))

(fn KillAI
  (bind _asbp_marine (Utilities|Casting|CastToBP_Marine (Game|GetPlayerCharacter 0)))
  (Default|IncreaseKills _asbp_marine)
  (bind _asbp_marine_game_mode (Utilities|Casting|CastToBP_MarineGameMode (Game|GetGameMode)))
  (Default|RegisterAlienDeath _asbp_marine_game_mode self)
  (Components|Activation|Deactivate (Variables|Character|GetCharacterMovement))
  (Components|DestroyComponent (Variables|Collision|GetCapsuleComponent)))