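; BP_Marine is the player marine, with world-axis movement, a HUD, health, a kill counter and a rifle that damages BP_Alien.
; Aim turns control yaw toward the direction of mouse velocity, smoothed and filtered by a deadzone.
; Holding fire runs a looping timer of line traces with particles and sound.
; Sprint temporarily boosts speed and grants damage immunity, then cools down; death stops firing and movement.
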(event EventTick
  (params (DeltaSeconds :type Float%20%28single-precision%29))
  (if (not (Variables|Default|GetIs%20Dead))
    (CallFunction|UpdatePlayerAim)))

(event EventBeginPlay
  (bind _returnvalue (UserInterface|CreateWidget "/Game/Blueprints/Pawns/Marine/UMG_HUD.UMG_HUD_C"))
  (UserInterface|Viewport|AddtoPlayerScreen _returnvalue))

(event Game|Damage|EventAnyDamage
  (params (Damage :type Float%20%28single-precision%29) (DamageType :type Damage%20Type%20Object%20Reference) (InstigatedBy :type Controller%20Object%20Reference) (DamageCauser :type Actor%20Object%20Reference))
  (if (not (Variables|Default|GetIs%20Immune%20To%20Damage))
    (Utilities|DamagePlayer Damage
      (:Player%20Is%20Dead
        (CallFunction|KillPlayer)))))

(event Input|ActionEvents|InputActionFire
  (params (Key :type Key%20Structure :default "None"))
  (:Pressed
    (if (not (Variables|Default|GetIs%20Dead))
      (CallFunction|StartFiring)))
  (:Released
    (if (not (Variables|Default|GetIs%20Dead))
      (CallFunction|StopFiring))))

(event Input|AxisEvents|InputAxisMoveForward
  (params (AxisValue :type Float%20%28single-precision%29))
  (Pawn|Input|AddMovementInput "1.000000, 0, 0" AxisValue false))

(event Input|AxisEvents|InputAxisMoveRight
  (params (AxisValue :type Float%20%28single-precision%29))
  (Pawn|Input|AddMovementInput "0.000000,1.000000, 0" AxisValue false))

(event Input|KeyboardEvents|LeftShift
  (params (Key :type Key%20Structure :default "None"))
  (:Pressed
    (Utilities|Sprint)))

(fn ConstructionScript)

(fn GetMouseVelocity
  (bind _returnvalue (Game|GetPlayerController 0))
  (bind (_deltax _deltay) (Class|PlayerController|GetInputMouseDelta _returnvalue))
  (return (/ (Math|Vector2D|MakeVector2D _deltax _deltay) (Utilities|Time|GetWorldDeltaSeconds))))

(fn UpdatePlayerAim
  (bind _mouse_velocity (CallFunction|GetMouseVelocity))
  (bind _returnvalue (Game|GetPlayerController 0))
  (if (CallFunction|IsMouseVelocityAboveDeadzone?)
    (Pawn|SetControlRotation _returnvalue (Math|Interpolation|RInterpTo (Pawn|GetControlRotation _returnvalue :!class /Script/Engine.Controller) (Math|Rotator|MakeRotator 0.0 0.0 (Class|KismetMathLibrary|DegAtan2 (.x _mouse_velocity) (.y _mouse_velocity))) (Utilities|Time|GetWorldDeltaSeconds) (Variables|Default|GetMouse%20Smoothing%20Strength)))))

(fn IsMouseVelocityAboveDeadzone?
  (return (> (Math|Vector2D|Vector2DLength (CallFunction|GetMouseVelocity)) (Variables|Default|GetMouse%20Deadzone))))

(fn StartFiring
  (Components|Activation|SetActive (Variables|Default|GetParticleSystem) true false)
  (bind _returnvalue (Audio|SpawnSound2D "/Game/Sounds/Weapon_AssaultRifle/Stereo/RifleFire_Cue.RifleFire_Cue" 1.0 1.0 0.0 0))
  (Variables|Default|SetFire%20sound _returnvalue)
  (Utilities|Time|SetTimerbyFunctionName 0 "Weapon Trace" (Variables|Default|GetWeapon%20fire%20rate) true))

(fn StopFiring
  (Components|Activation|SetActive (Variables|Default|GetParticleSystem) false false)
  (bind _fire_sound (Variables|Default|GetFire%20sound)
    (:then
      (Audio|Components|Audio|Stop _fire_sound)
      (Utilities|Time|ClearTimerbyFunctionName 0 "Weapon Trace")
      (if (not (Variables|Default|GetIs%20Dead))
        (Audio|SpawnSound2D "/Game/Sounds/Weapon_AssaultRifle/Stereo/RifleFireEnd_Cue.RifleFireEnd_Cue" 1.0 1.0 0.0 0)))
    (:else)))

(fn WeaponTrace
  (bind _returnvalue (Transformation|GetActorLocation))
  (bind _outhit (Collision|LineTraceByChannel _returnvalue (+ _returnvalue (* (Transformation|GetActorForwardVector) 7e+02)) "TraceTypeQuery1" false 0 "None"))
  (Effects|SpawnEmitteratLocation "/Game/Effects/Weapons/Impacts/P_AssaultRifle_IH.P_AssaultRifle_IH" (.location _outhit))
  (if (== (Utilities|GetClass (.hitactor _outhit)) "/Game/Blueprints/Pawns/Alien/BP_Alien.BP_Alien_C")
    (Game|Damage|ApplyDamage (.hitactor _outhit) (Variables|Default|GetShot%20Damage) 0 0)))

(fn IncreaseKills
  (bind _result (Math|Integer|IncrementInt (Variables|Default|GetAliens%20Killed))
    (:%20%20
      (Variables|Default|SetAliens%20Killed _result))))

(fn AddHealth
  (params (Health%20to%20Add :type Float%20%28single-precision%29))
  (Variables|Default|SetHealth (Math|Float|Clamp(Float) (+ Health%20to%20Add (Variables|Default|GetHealth)) 0.0 1e+02)))

(fn IsHealthFull?
  (return (== (Variables|Default|GetHealth) 1e+02)))

(fn KillPlayer
  (Variables|Default|SetIs%20Dead true)
  (CallFunction|StopFiring)
  (Components|Activation|Deactivate (Variables|Character|GetCharacterMovement)))