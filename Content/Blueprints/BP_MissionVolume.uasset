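; BP_MissionVolume is a box volume that bounds the mission area and kills the player for staying outside it.
; When a BP_Marine exits the box, it sets that marine's OutsideMissionArea flag and starts a Kill Player timer lasting KillDelayTime.
; Re-entering clears the flag and the timer.
; On expiry, the timer applies massive damage to player character 0, not necessarily the marine that left.
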(event OnComponentBeginOverlap(Box)
  (params (OverlappedComponent :type Primitive%20Component%20Object%20Reference) (OtherActor :type Actor%20Object%20Reference) (OtherComp :type Primitive%20Component%20Object%20Reference) (OtherBodyIndex :type Integer) (bFromSweep :type Boolean) (SweepResult :type Hit%20Result%20Structure%20%28by%20ref%29))
  (bind _asbp_marine (Utilities|Casting|CastToBP_Marine OtherActor))
  (Variables|/Game/Blueprints/Pawns/Marine/BP_Marine.BP_Marine_C|SetOutside%20Mission%20Area _asbp_marine false)
  (Utilities|Time|ClearTimerbyFunctionName 0 "Kill Player"))

(event OnComponentEndOverlap(Box)
  (params (OverlappedComponent :type Primitive%20Component%20Object%20Reference) (OtherActor :type Actor%20Object%20Reference) (OtherComp :type Primitive%20Component%20Object%20Reference) (OtherBodyIndex :type Integer))
  (bind _asbp_marine (Utilities|Casting|CastToBP_Marine OtherActor))
  (Variables|/Game/Blueprints/Pawns/Marine/BP_Marine.BP_Marine_C|SetOutside%20Mission%20Area _asbp_marine true)
  (Utilities|Time|SetTimerbyFunctionName 0 "Kill Player" (Variables|Default|GetKill%20Delay%20Time)))

(event Custom|Kill%20Player
  (Game|Damage|ApplyDamage (Game|GetPlayerCharacter 0) 1e+04 0 0))

(event EventBeginPlay)

(fn ConstructionScript)